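; BP_Cube is a damageable, healable cube actor that delegates its health logic to a DamageSystem component.
; Heal, TakeDamage and the current health, max health and death queries are thin wrappers that forward to that component.
; TakeDamage also prints the resulting health as debug output before returning the component's result.
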(event EventBeginPlay)

(event Collision|EventActorBeginOverlap
  (params (OtherActor :type Actor%20Object%20Reference)))

(event EventTick
  (params (DeltaSeconds :type Float%20%28single-precision%29)))

(event EventHeal
  (params (HealAmount :type Float%20%28single-precision%29) (Healer :type Actor%20Object%20Reference))
  (Class|DamageSystemComponent|HandleIncomingHeal (Variables|Default|GetDamageSystem) HealAmount Healer))

(fn ConstructionScript)

(fn GetCurrentHealth
  (return (Class|DamageSystemComponent|GetCurrentHealth (Variables|Default|GetDamageSystem))))

(fn GetIsDead
  (return (Class|DamageSystemComponent|GetIsDead (Variables|Default|GetDamageSystem))))

(fn GetMaxHealth
  (return (Class|DamageSystemComponent|GetMaxHealth (Variables|Default|GetDamageSystem))))

(fn TakeDamage
  (params (DamageInfo :type Damage%20Info%20Structure%20%28by%20ref%29))
  (bind _returnvalue (Class|DamageSystemComponent|HandleIncomingDamage (Variables|Default|GetDamageSystem) DamageInfo))
  (bind _returnvalue_2 (CallFunction|GetCurrentHealth))
  (Development|PrintString (Utilities|String|ToString(Float) _returnvalue_2))
  (return _returnvalue))