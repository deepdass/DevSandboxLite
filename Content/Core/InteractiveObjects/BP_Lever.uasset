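; BP_Lever is an interactive lever that triggers linked actors when pulled.
; Interact flip-flops the LeverPullPitch timeline forward and in reverse to rotate the handle mesh.
; Each timeline update adds the Keycard gameplay tag to the instigator's SActionComponent tags.
; When the timeline finishes in either direction, it sends Interact to SelectedActor and remotely detonates SelectedActor0 if that is a BP_Explosivebarrel.
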(event EventBeginPlay)

(event Collision|EventActorBeginOverlap
  (params (OtherActor :type Actor%20Object%20Reference)))

(event EventTick
  (params (DeltaSeconds :type Float%20%28single-precision%29)))

(event EventInteract
  (params (InstigatorPawn :type Pawn%20Object%20Reference))
  (Utilities|FlowControl|FlipFlop
    (:A
      (bind _newtrack_0 (Timeline|Lever%20pull%20pitch Play)
        (:Update
          (Transformation|SetRelativeRotation (Variables|Default|GetHandleMesh) (Math|Rotator|MakeRotator 0.0 _newtrack_0 0.0) false false)
          (GameplayTags|AddGameplayTag (Variables|/Script/Projectidk.SActionComponent|GetActiveGameplayTags (Actor|GetComponentbyClass InstigatorPawn "/Script/Projectidk.SActionComponent")) (Variables|Default|GetKeycard) :!class /Script/GameplayTags.BlueprintGameplayTagLibrary))
        (:Finished
          (Class|SGameplayInterface|Interact(Message) (Variables|Default|GetSelectedActor) InstigatorPawn)
          (bind _asbp_explosivebarrel (Utilities|Casting|CastToBP_Explosivebarrel (Variables|Default|GetSelectedActor_0)))
          (Default|Explodefromdistance _asbp_explosivebarrel))))
    (:B
      (Timeline|Lever%20pull%20pitch Reverse))))

(fn ConstructionScript)