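; BP_PhysicsCube is an interactive-object cube that gets a random, fully saturated color when play begins.
; The server picks a random hue on BeginPlay, stores it in the replicated CubeColor and applies it to the mesh materials' BaseColor parameter.
; Clients apply the same color through the CubeColor OnRep, so the color is synced as state rather than by RPC.
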(event Custom|SetCubeColor
  (params (Color :type Linear%20Color%20Structure))
  (Rendering|Material|SetVectorParameterValueonMaterials (Variables|Default|GetCube) "BaseColor" (Math|Conversions|ToVector(LinearColor) Color)))

(event EventBeginPlay
  (if (Ability|HasAuthority)
    (bind _output_get (Variables|Default|SetCubeColor (Class|KismetMathLibrary|HSVtoRGB (Math|Random|RandomFloatinRange 0.0 3.6e+02) 1.0 1.0 1.0)))
    (CallFunction|SetCubeColor _output_get)))

(fn ConstructionScript)

(fn OnRepCubeColor
  (CallFunction|SetCubeColor (Variables|Default|GetCubeColor)))